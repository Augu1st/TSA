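; BP_TestActor is a test item actor that supplies hint, prompt and state hooks for interaction.
; ShowHint and HideHint toggle custom depth rendering on its Cube, while ShowPrompt and HidePrompt toggle the visibility of its Prompt component.
; GetInteractState is a stub returning None, and the default BeginPlay, overlap and Tick events are unused.
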(event EventBeginPlay)

(event Collision|EventActorBeginOverlap
  (params (OtherActor :type Actor%20Object%20Reference)))

(event EventTick
  (params (DeltaSeconds :type Float%20%28single-precision%29)))

(event EventShowHint
  (Rendering|SetRenderCustomDepth (Variables|Default|GetCube) true))

(event EventHideHint
  (Rendering|SetRenderCustomDepth (Variables|Default|GetCube) false))

(event EventShowPrompt
  (Rendering|SetVisibility (Variables|Default|GetPrompt) true false))

(event EventHidePrompt
  (Rendering|SetVisibility (Variables|Default|GetPrompt) false false))

(fn ConstructionScript)

(fn GetInteractState
  (return "None"))