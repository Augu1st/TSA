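; BP_TestActor is a test item actor that the player can interact with to pick up.
; On BeginPlay it sets an F-key icon and text on its prompt widget.
; Interaction events toggle that prompt's visibility and highlight the mesh through custom depth rendering.
; PrimaryInteract casts the interactor to TSA_PlayerController and requests pickup of its item component, while GetInteractState reports Interactable.
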(event EventBeginPlay
  (bind _aswbp_tsa_interact_prompt_widget (Utilities|Casting|CastToWBP_TSA_InteractPromptWidget (UserInterface|GetWidget (Variables|Default|GetPrompt))))
  (Class|TSAPromptWidget|SetKeyImage _aswbp_tsa_interact_prompt_widget (Utilities|Struct|MakeSlateBrush "(SpecifiedColor=(R=1.000000,G=1.000000,B=1.000000,A=1.000000),ColorUseRule=UseColor_Specified)" "Image" "NoTile" "NoMirror" "(X=32.000000,Y=32.000000)" "(Left=0.000000,Top=0.000000,Right=0.000000,Bottom=0.000000)" "/Game/Assets/UI/EasyInputPrompts/GraphicContent/MouseAndKeyboard/T_Keyboard_F.T_Keyboard_F" "(CornerRadii=(X=0.000000,Y=0.000000,Z=0.000000,W=0.000000),Color=(SpecifiedColor=(R=0.000000,G=0.000000,B=0.000000,A=0.000000),ColorUseRule=UseColor_Specified),Width=0.000000,RoundingType=HalfHeightRadius,bUseBrushTransparency=False)"))
  (Class|TSAPromptWidget|SetPromptText _aswbp_tsa_interact_prompt_widget (Variables|Default|GetText)))

(event Collision|EventActorBeginOverlap
  (params (OtherActor :type Actor%20Object%20Reference)))

(event EventTick
  (params (DeltaSeconds :type Float%20%28single-precision%29)))

(event EventShowHint
  (Rendering|SetRenderCustomDepth (Variables|Default|GetStaticMesh) true))

(event EventHideHint
  (Rendering|SetRenderCustomDepth (Variables|Default|GetStaticMesh) false))

(event EventShowPrompt
  (Rendering|SetVisibility (Variables|Default|GetPrompt) true false))

(event EventHidePrompt
  (Rendering|SetVisibility (Variables|Default|GetPrompt) false false))

(event EventPrimaryInteract
  (params (Interactor :type Player%20Controller%20Object%20Reference))
  (bind _astsa_player_controller (Utilities|Casting|CastToTSA_PlayerController Interactor))
  (Class|TSAPlayerController|RequestPickUpItem _astsa_player_controller (Variables|Default|GetBP_TSA_ItemComponent)))

(fn ConstructionScript)

(fn GetInteractState
  (return "Interactable"))